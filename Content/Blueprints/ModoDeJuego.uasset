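; Game mode Blueprint that picks the player's spawn point from a flag name held by the game instance.
; Its ChoosePlayerStart override returns the PlayerStart whose PlayerStartTag matches the flag name from CustomGameInstance.
; If the game instance cast fails, it returns the first PlayerStart found, but an unmatched tag has no fallback.
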(event EventBeginPlay)

(event EventTick
  (params (DeltaSeconds :type Float%20%28single-precision%29)))

(fn ConstructionScript)

(fn ChoosePlayerStart
  (params (Player :type Controller%20Object%20Reference))
  (bind _ascustom_game_instance (Utilities|Casting|CastToCustomGameInstance (Game|GetGameInstance))
    (:then
      (bind _outactors (Actor|GetAllActorsOfClass "/Script/Engine.PlayerStart"))
      (for _array_element _outactors
        (if (Utilities|Name|Equal(Name) (Variables|/Script/Engine.PlayerStart|GetPlayerStartTag _array_element) (Default|GetFlagName _ascustom_game_instance))
          (return _array_element))))
    (:CastFailed
      (bind _returnvalue (Actor|GetActorOfClass "/Script/Engine.PlayerStart"))
      (return _returnvalue))))