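; A moving platform that shuttles a Paper2D tile map back and forth through the points of a spline.
; A timeline lerps the tile map from its current world location to the target spline point, taking the same timeline duration for every segment.
; When each move finishes, it steps the point index and starts the next move, reversing direction at either end of the spline.
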(event Custom|MoveToNextPoint
  (params (PointIndex :type Integer))
  (bind _plataformas1 (Variables|Default|GetPlataformas1))
  (Variables|Default|SetPreLocation (Transformation|GetWorldLocation _plataformas1))
  (bind _alpha (Timeline|MovePlatform PlayFromStart)
    (:Update
      (Transformation|SetWorldLocation _plataformas1 (Math|Vector|Lerp(Vector) (Variables|Default|GetPreLocation) (.Location (Math|Transform|BreakTransform (Spline|GetTransformatSplinePoint (Variables|Default|GetSpline) PointIndex "World" false))) _alpha) false false))
    (:Finished
      (if (Variables|Default|GetReversing)
        (if (< (- (Variables|Default|GetCurrentPointIndex) 1) 0)
          (Variables|Default|SetReversing false))
        (elif (>= (+ (Variables|Default|GetCurrentPointIndex) 1) (Spline|GetNumberOfSplinePoints (Variables|Default|GetSpline)))
          (Variables|Default|SetReversing true)))
      (if (Variables|Default|GetReversing)
        (CallFunction|MovetoNextPoint (+ (Variables|Default|GetCurrentPointIndex) -1))
        (Variables|Default|SetCurrentPointIndex (+ (Variables|Default|GetCurrentPointIndex) -1))
        (else
          (CallFunction|MovetoNextPoint (+ (Variables|Default|GetCurrentPointIndex) 1))
          (Variables|Default|SetCurrentPointIndex (+ (Variables|Default|GetCurrentPointIndex) 1)))))))

(event EventBeginPlay
  (CallFunction|MovetoNextPoint (Variables|Default|GetCurrentPointIndex))
  (Class|PaperTileMapComponent|SetTileMap (Variables|Default|GetPlataformas1) "/Game/Texturas/Terrain/MovPlatform1.MovPlatform1"))

(fn ConstructionScript
  (Class|PaperTileMapComponent|SetTileMap (Variables|Default|GetPlataformas1) "/Game/Texturas/Terrain/MovPlatform1.MovPlatform1"))